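; Player Blueprint that handles fixed-step vertical looking and a toggleable codex screen through Enhanced Input.
; BeginPlay adds the controls mapping context; look up and down inputs snap control pitch between level, raised and lowered views, preserving yaw.
; The codex toggle creates a fresh widget and shows the cursor, or removes all widgets and hides it.
; Mouse look is empty, and the HUD, garnish and ingredient widget setup is unconnected.
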(event Input|EnhancedActionEvents|EnhancedInputActionIA_MouseLook
  (params (ActionValue :type Float%20%28double-precision%29) (ElapsedSeconds :type Float%20%28double-precision%29) (TriggeredSeconds :type Float%20%28double-precision%29) (InputAction :type Input%20Action%20Object%20Reference :default "/Game/Input/IA_MouseLook.IA_MouseLook"))
  ;[0 0.15 0.136 0.5] Mouse Look Around
)

(event Input|EnhancedActionEvents|EnhancedInputActionIA_LookUp
  (params (ActionValue :type Float%20%28double-precision%29) (ElapsedSeconds :type Float%20%28double-precision%29) (TriggeredSeconds :type Float%20%28double-precision%29) (InputAction :type Input%20Action%20Object%20Reference :default "/Game/Input/IA_LookUp.IA_LookUp"))
  (bind _returnvalue (Pawn|GetControlRotation :!class /Script/Engine.Pawn))
  (bind _yaw (Math|Rotator|BreakRotator _returnvalue))
  ;[0.03518 0.15 0 0.5] LookUp (W)
  (:Started
    (if (== (Variables|Default|GetCurrentView) 2)
      (Pawn|SetControlRotation (Game|GetPlayerController 0) (Math|Rotator|MakeRotator 0.0 0.0 _yaw))
      (Variables|Default|SetCurrentView 0)
      (else
        (Pawn|SetControlRotation (Game|GetPlayerController 0) (Math|Rotator|MakeRotator 0.0 3e+01 _yaw))
        (Variables|Default|SetCurrentView 1)))))

(event Input|EnhancedActionEvents|EnhancedInputActionIA_ToggleCodex
  (params (ActionValue :type Boolean) (ElapsedSeconds :type Float%20%28double-precision%29) (TriggeredSeconds :type Float%20%28double-precision%29) (InputAction :type Input%20Action%20Object%20Reference :default "/Game/Input/IA_ToggleCodex.IA_ToggleCodex"))
  ;[0.1106 0.08182 0.15 0.5] Codex Toggle
  (:Started
    (if (Variables|Default|GetIsCodexOpen)
      (Viewport|RemoveAllWidgets)
      (Variables|Default|SetIsCodexOpen false)
      (Variables|/Script/Engine.PlayerController|SetbShowMouseCursor (Game|GetPlayerController 0) false)
      (else
        (bind _returnvalue (UserInterface|CreateWidget "/Game/UI/WBP_Codex.WBP_Codex_C" (Game|GetPlayerController 0)))
        (bind _output_get (Variables|Default|SetCodexWidget _returnvalue))
        (UserInterface|Viewport|AddtoViewport _output_get 0)
        (Variables|Default|SetIsCodexOpen true)
        (Variables|/Script/Engine.PlayerController|SetbShowMouseCursor (Game|GetPlayerController 0) true)))))

(event Input|EnhancedActionEvents|EnhancedInputActionIA_LookDown
  (params (ActionValue :type Float%20%28double-precision%29) (ElapsedSeconds :type Float%20%28double-precision%29) (TriggeredSeconds :type Float%20%28double-precision%29) (InputAction :type Input%20Action%20Object%20Reference :default "/Game/Input/IA_LookDown.IA_LookDown"))
  (bind _returnvalue (Pawn|GetControlRotation :!class /Script/Engine.Pawn))
  (bind _yaw (Math|Rotator|BreakRotator _returnvalue))
  ;[0.1486 0.15 0.000259 0.5] Look Down (S)
  (:Started
    (if (== (Variables|Default|GetCurrentView) 1)
      (Pawn|SetControlRotation (Game|GetPlayerController 0) (Math|Rotator|MakeRotator 0.0 0.0 _yaw))
      (Variables|Default|SetCurrentView 0)
      (else
        (Pawn|SetControlRotation (Game|GetPlayerController 0) (Math|Rotator|MakeRotator 0.0 -25.0 _yaw))
        (Variables|Default|SetCurrentView 2)))))

(event EventBeginPlay
  (CallFunction|SetupInput)
  (bind _returnvalue (UserInterface|CreateWidget "/Game/UI/WBP_Codex.WBP_Codex_C"))
  (Variables|Default|SetCodexWidget _returnvalue))

(fn ConstructionScript)

(fn SetupInput
  (Input|AddMappingContext (PlayerController|LocalPlayerSubsystems|GetEnhancedInputLocalPlayerSubsystem (Game|GetPlayerController 0)) "/Game/Input/IMC_Controls.IMC_Controls" 0 "(bIgnoreAllPressedKeysUntilRelease=True,bForceImmediately=False,bNotifyUserSettings=False)"))